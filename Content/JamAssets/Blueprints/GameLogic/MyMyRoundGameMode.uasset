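; Game mode that tracks enemy waves in a round-based game, counting spawned and killed enemies, with kills capped at the round maximum.
; At BeginPlay it gathers all BP_MySpawner actors and binds to a round-ended callback.
; When a round ends it resets counters, scales up the HP factor and enemy cap, clears the enemy list and flags every spawner.
; Tick prints debug counts, and several events are empty stubs.
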(event `self.ReceiveBeginPlay`
  (add `self.OnRoundEndedCallback` (delegate `OnRoundFinished`))
  (bind _outactors (`GameplayStatics.GetAllActorsOfClass` "/Game/JamAssets/Blueprints/GameLogic/BP_MySpawner.BP_MySpawner_C"))
  (set `self.Spawners` _outactors))

(event `OnRoundFinished`
  (`/Engine/EditorBlueprintResources/StandardMacros.IncrementInt` (`self.CurrentRound`)
    (:`  `
      (set `self.EnemiesKilled` 0)
      (set `self.EnemiesSpawned` 0)
      (set `self.HpIncreaseFactor` (* (`self.HpIncreaseFactor`) 1.2))
      (set `self.MaxEnemiesPerRound` (+ (`self.MaxEnemiesPerRound`) 5))
      (`KismetArrayLibrary.Array_Clear` (`self.Enemies`))
      (for _array_element (`self.Spawners`)
        (set `/Game/JamAssets/Blueprints/GameLogic/BP_MySpawner.IsNewRound` true _array_element)))))

(event `WaitTimeEnded`)

(event `OnEnemyKilled`
  (bind _maxenemiesperround (`self.MaxEnemiesPerRound`))
  (bind _result (`/Engine/EditorBlueprintResources/StandardMacros.IncrementInt` (`self.EnemiesKilled`))
    (:`  `
      (if (>= _result _maxenemiesperround)
        (set `self.EnemiesKilled` _maxenemiesperround)))))

(event `self.ReceiveTick`
  (params (DeltaSeconds :type "Float (single-precision)"))
  (`KismetSystemLibrary.PrintString` (`KismetStringLibrary.Conv_IntToString` (`KismetArrayLibrary.Array_Length` (`self.Enemies`))))
  (`KismetSystemLibrary.PrintText` (`|FormatText` "Enemies Killed :::{n}" (`self.EnemiesKilled`))))

(event `OnMaxEnemiesIncrease`)

(event `OnEnemySpawned`
  (`/Engine/EditorBlueprintResources/StandardMacros.IncrementInt` (`self.EnemiesSpawned`)))

(event `AddRound`)

(fn `UserConstructionScript`)