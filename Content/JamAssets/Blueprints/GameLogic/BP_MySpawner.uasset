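; BP_MySpawner is a spawner actor that spawns one configured enemy type (Healer, Normal or Floating Head) at its location during rounds.
; Tick reads spawn and kill counts from MyMyRoundGameMode, reporting each spawn until the round limit and calling the round-ended callback once kills reach it.
; Delay nodes on Tick pace spawns by SpawnRate and hold a pause while IsNewRound is set.
; An alternative round-end check remains unconnected.
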(event `self.ReceiveBeginPlay`
  (bind _asmy_my_round_game_mode (cast `/Game/JamAssets/Blueprints/GameLogic/MyMyRoundGameMode` (`GameplayStatics.GetGameMode`)))
  (set `self.My My Round Game Mode` _asmy_my_round_game_mode))

(event `self.ReceiveTick`
  (params (DeltaSeconds :type "Float (single-precision)"))
  (bind _my_my_round_game_mode (`self.My My Round Game Mode`))
  (bind _returnvalue (`KismetMathLibrary.Conv_VectorToTransform` (`self.K2_GetActorLocation`)))
  (if (`self.IsNewRound`)
    (`KismetSystemLibrary.Delay` 10.0)
    (set `self.IsNewRound` false)
    (elif (>= (`MyRoundGameMode.EnemiesKilled` (`self.My My Round Game Mode`)) (`MyRoundGameMode.MaxEnemiesPerRound` (`self.My My Round Game Mode`)))
      (`/Game/JamAssets/Blueprints/GameLogic/MyMyRoundGameMode.OnRoundEndedCallback` (`self.My My Round Game Mode`))
      (elif (< (`MyRoundGameMode.EnemiesSpawned` _my_my_round_game_mode) (`MyRoundGameMode.MaxEnemiesPerRound` _my_my_round_game_mode))
        (`KismetSystemLibrary.Delay` (`self.SpawnRate`))
        (`KismetSystemLibrary.PrintString` (`KismetStringLibrary.Conv_IntToString` (`MyRoundGameMode.EnemiesSpawned` (`self.My My Round Game Mode`))))
        (`/Game/JamAssets/Blueprints/GameLogic/MyMyRoundGameMode.OnEnemySpawned` _my_my_round_game_mode)
        (switch `/Game/JamAssets/Blueprints/ENUM/E_SpawnType` (`self.EnemyType`)
          (:`NewEnumerator0`
            (`|SpawnActorFromClass` "/Game/JamAssets/Blueprints/AI/BP_Healer.BP_Healer_C" _returnvalue "Undefined" "MultiplyWithRoot" null null))
          (:`NewEnumerator1`
            (`|SpawnActorFromClass` "/Game/JamAssets/Blueprints/AI/BP_Normal.BP_Normal_C" _returnvalue "Undefined" "MultiplyWithRoot" null null))
          (:`NewEnumerator2`
            (`|SpawnActorFromClass` "/Game/JamAssets/Blueprints/AI/BP_FloatHead.BP_FloatHead_C" _returnvalue "Undefined" "MultiplyWithRoot" null null)))))))

(fn `UserConstructionScript`)