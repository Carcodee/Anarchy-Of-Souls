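; Floating damage text actor that shows a damage number on a WB_FloatingText widget, drifts away and then removes itself.
; BeginPlay passes the color and ScreenDamage to the widget, and the MoveTo timeline lerps the actor toward a fixed world-space offset, destroying it on finish.
; Tick rotates the whole actor with LookAt to keep it facing the player pawn, rather than the camera.
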(event `self.ReceiveBeginPlay`
  (bind _aswb_floating_text (cast `/Game/JamAssets/Blueprints/Widgets/WB_FloatingText` (`WidgetComponent.GetWidget` (`self.Widget`))))
  (`UserWidget.SetColorAndOpacity` _aswb_floating_text (`self.In Color and Opacity`))
  (set `/Game/JamAssets/Blueprints/Widgets/WB_FloatingText.Damage` (`self.ScreenDamage`) _aswb_floating_text)
  (bind _output_get (set `self.StartLoc` (`self.K2_GetActorLocation`)))
  (set `self.EndLoc` (+ _output_get (-25.0 250.0 250.0)))
  (bind (_direction _move_track) (`Timeline|Move to`)
    (:`Update`
      (`self.K2_SetActorLocation` (`KismetMathLibrary.VLerp` (`self.StartLoc`) (`self.EndLoc`) _move_track)))
    (:`Finished`
      (`self.K2_DestroyActor`))))

(event `self.ReceiveTick`
  (params (DeltaSeconds :type "Float (single-precision)"))
  (`self.K2_SetActorTransform` (`KismetAnimationLibrary.K2_LookAt` (`self.GetTransform`) (`self.K2_GetActorLocation` (`GameplayStatics.GetPlayerPawn` 0)) (1.0 0.0 0.0) false (0.0 0.0 1.0))))

(fn `UserConstructionScript`)