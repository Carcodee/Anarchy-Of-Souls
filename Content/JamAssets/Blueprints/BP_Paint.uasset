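; BP_Paint is a damage zone that hurts the player or an enemy overlapping its Box.
; Begin overlap accepts Tickeable actors, storing the latest player or enemy and setting flags; IsPlayerInside covers both.
; Every frame, Tick sends enemies TickDamageMessage and MakeDamage using random player damage ranges, or sends the player DamageDone and signals a health change.
; End overlap's interface check has no object connected, so its flag reset appears unreachable.
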(event `self.ReceiveTick`
  (params (DeltaSeconds :type "Float (single-precision)"))
  (bind _as_bp_first_person_character (`self.As BP First Person Character`))
  (bind _as_bp_my_normal_enemy_aibase (`self.As BP My Normal Enemy AIBase`))
  (if (`self.IsPlayerInside`)
    (if (`self.EnemyInside`)
      (if (`KismetSystemLibrary.IsValid` _as_bp_my_normal_enemy_aibase)
        (bind _asbp_first_person_character (cast `/Game/JamAssets/Blueprints/BP_FirstPersonCharacter` (`GameplayStatics.GetPlayerPawn` 0)))
        (bind _returnvalue (`KismetMathLibrary.RandomIntegerInRange` (`JamCharacter.MinDamage` _asbp_first_person_character) (`JamCharacter.MaxDamage` _asbp_first_person_character)))
        (message `Tickeable.TickDamage` _as_bp_my_normal_enemy_aibase _returnvalue)
        (`/Engine/EditorBlueprintResources/StandardMacros.IsValid` _as_bp_my_normal_enemy_aibase
          (:`Is Valid`
            (`/Game/JamAssets/Blueprints/AI/BP_MyNormalEnemyAIBase.MakeDamage` _as_bp_my_normal_enemy_aibase (0.0 0.0 0.0) _returnvalue))))
      (else
        (message `Tickeable.TickDamage` _as_bp_first_person_character (`self.DamageDone`))
        (`/Game/JamAssets/Blueprints/BP_FirstPersonCharacter.OnHealthChanged` _as_bp_first_person_character)))))

(event `self.Box.OnComponentBeginOverlap`
  (params (OverlappedComponent :type "PrimitiveComponent Object Reference") (OtherActor :type "Actor Object Reference") (OtherComp :type "PrimitiveComponent Object Reference") (OtherBodyIndex :type Integer) (bFromSweep :type Boolean) (SweepResult :type "HitResult Structure (by ref)"))
  (if (`KismetSystemLibrary.DoesImplementInterface` OtherActor "/Script/Jam.Tickeable")
    (bind _asbp_first_person_character (cast `/Game/JamAssets/Blueprints/BP_FirstPersonCharacter` OtherActor)
      (:`then`
        (set `self.As BP First Person Character` _asbp_first_person_character)
        (set `self.EnemyInside` false)
        (set `self.IsPlayerInside` true))
      (:`CastFailed`
        (bind _asbp_my_normal_enemy_aibase (cast `/Game/JamAssets/Blueprints/AI/BP_MyNormalEnemyAIBase` OtherActor))
        (set `self.As BP My Normal Enemy AIBase` _asbp_my_normal_enemy_aibase)
        (set `self.IsPlayerInside` true)
        (set `self.EnemyInside` true)))))

(event `self.Box.OnComponentEndOverlap`
  (params (OverlappedComponent :type "PrimitiveComponent Object Reference") (OtherActor :type "Actor Object Reference") (OtherComp :type "PrimitiveComponent Object Reference") (OtherBodyIndex :type Integer))
  (if (`KismetSystemLibrary.DoesImplementInterface` null "/Script/Jam.Tickeable")
    (set `self.IsPlayerInside` false)))

(fn `UserConstructionScript`)