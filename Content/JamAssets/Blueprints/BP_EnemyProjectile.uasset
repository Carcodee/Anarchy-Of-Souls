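; BP_EnemyProjectile is an enemy projectile that damages the first-person player character on contact.
; Each Tick offsets the root along the normalized Dir vector by Speed, without sweep or delta-time scaling, so movement depends on frame rate.
; An overlap on the Projectile component applies Damage to BP_FirstPersonCharacter and destroys the actor.
; Other overlaps are ignored, and a short lifespan set at BeginPlay removes projectiles that miss.
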(event `self.ReceiveBeginPlay`
  (`self.SetLifeSpan` 5.0))

(event `self.ReceiveActorBeginOverlap`
  (params (OtherActor :type "Actor Object Reference")))

(event `self.ReceiveTick`
  (params (DeltaSeconds :type "Float (single-precision)"))
  (`SceneComponent.K2_AddWorldOffset` (`self.DefaultSceneRoot`) (* (`KismetMathLibrary.GetForwardVector` (`KismetMathLibrary.Conv_VectorToRotator` (`self.Dir`))) (`self.speed`)) false false))

(event `self.projectile.OnComponentBeginOverlap`
  (params (OverlappedComponent :type "PrimitiveComponent Object Reference") (OtherActor :type "Actor Object Reference") (OtherComp :type "PrimitiveComponent Object Reference") (OtherBodyIndex :type Integer) (bFromSweep :type Boolean) (SweepResult :type "HitResult Structure (by ref)"))
  (bind _asbp_first_person_character (cast `/Game/JamAssets/Blueprints/BP_FirstPersonCharacter` OtherActor))
  (`/Game/JamAssets/Blueprints/BP_FirstPersonCharacter.TakeDamage` _asbp_first_person_character (`self.Damage`))
  (`self.K2_DestroyActor`))

(fn `UserConstructionScript`)