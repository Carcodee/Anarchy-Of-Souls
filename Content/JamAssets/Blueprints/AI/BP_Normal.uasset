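; BP_Normal is an AI enemy that chases and punches the player, setting the IsChasing blackboard key on BeginPlay.
; OnAttackPlayer checks player distance, sphere-traces forward, then applies damage to the first-person character and signals its health change.
; Damage events spawn floating text actors, either delayed or instantly.
; MakeFloatingDamage, uncalled here, builds numbers from per-digit Niagara systems, while Attack is a stub returning zero.
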(event `self.ReceiveBeginPlay`
  (bind _asbp_first_person_character (cast `/Game/JamAssets/Blueprints/BP_FirstPersonCharacter` (`GameplayStatics.GetPlayerPawn` 0)))
  (set `self.As BP First Person Character` _asbp_first_person_character)
  (`BlackboardComponent.SetValueAsBool` (`AIBlueprintHelperLibrary.GetBlackboard` (`AIBlueprintHelperLibrary.GetAIController` self)) "IsChasing" true))

(event `self.ReceiveTick`
  (params (DeltaSeconds :type "Float (single-precision)"))
  (if (not (`self.IsTickeable`))
    (`KismetSystemLibrary.Delay` 0.8)
    (set `self.IsTickeable` true)))

(event `OnAttackPlayer`
  (bind _returnvalue (`self.K2_GetActorLocation`))
  (if (<= (`self.GetDistanceTo` (`GameplayStatics.GetPlayerPawn` 0)) 250.0)
    (bind (_outhit _returnvalue_2) (`KismetSystemLibrary.SphereTraceSingleForObjects` :`Start` _returnvalue :`End` (+ _returnvalue (* (`KismetMathLibrary.GetForwardVector` (`self.K2_GetActorRotation`)) (`self.AttackDistance`))) :`Radius` 120.0 :`ObjectTypes` (`|MakeArray` "ObjectTypeQuery3" :!type "EObjectTypeQuery Enum") :`DrawDebugType` "ForOneFrame"))
    (if _returnvalue_2
      (bind _asbp_first_person_character (cast `/Game/JamAssets/Blueprints/BP_FirstPersonCharacter` (`.HitActor` (`GameplayStatics.BreakHitResult` _outhit))))
      (set `self.IsEnemyPunching` false)
      (`/Game/JamAssets/Blueprints/BP_FirstPersonCharacter.TakeDamage` _asbp_first_person_character (`self.EnemyDamage`))
      (`/Game/JamAssets/Blueprints/BP_FirstPersonCharacter.OnHealthChanged` (`self.As BP First Person Character`)))
    (else
      (set `self.IsEnemyPunching` false))))

(event `MakeDamage`
  (params (Location :type "Vector Structure") (Amount :type Integer) (color :type "LinearColor Structure"))
  (`KismetSystemLibrary.Delay` 0.8)
  (`|SpawnActorFromClass` "/Game/JamAssets/Blueprints/HUDBP/BP_FloatingTextA.BP_FloatingTextA_C" (`self.GetTransform`) "Undefined" "MultiplyWithRoot" null Amount color null))

(event `InstantFloatingText`
  (params (Location :type "Vector Structure") (Amount :type Integer) (color :type "LinearColor Structure"))
  (`|SpawnActorFromClass` "/Game/JamAssets/Blueprints/HUDBP/BP_FloatingTextA.BP_FloatingTextA_C" (`self.GetTransform`) "Undefined" "MultiplyWithRoot" null Amount color null))

(fn `Attack`
  (returns (AnimationDecoration :type "Float (double-precision)"))
  (return 0.0))

(fn `MakeFloatingDamage`
  (params (Position :type "Vector Structure") (Amount :type Integer))
  (locals (DigitSystem :type "NiagaraComponent Object Reference") (YLocalOFfset :type "Float (double-precision)" :default 100.0))
  (bind (_returnvalue_roll _returnvalue_pitch _returnvalue_yaw) (`KismetMathLibrary.BreakRotator` (`Controller.GetControlRotation` (`GameplayStatics.GetPlayerController` 0))))
  (for _array_element (`KismetStringLibrary.GetCharacterArrayFromString` (`KismetStringLibrary.Conv_IntToString` Amount))
    (bind _returnvalue (`NiagaraFunctionLibrary.SpawnSystemAtLocation` "/Game/JamAssets/VFX/NE_FloatingNumbers_System.NE_FloatingNumbers_System" Position (`KismetMathLibrary.MakeRotator` 0.0 180.0 _returnvalue_yaw)))
    (bind _output_get (set `local.DigitSystem` _returnvalue))
    (`SceneComponent.K2_AddLocalOffset` _output_get (`KismetMathLibrary.MakeVector` 0.0 (`local.YLocalOFfset`)) false false)
    (set `local.YLocalOFfset` (+ (`local.YLocalOFfset`) 50.0))
    (switch `string` _array_element
      (:`Case_0`
        (`NiagaraFunctionLibrary.SetTextureObject` (`local.DigitSystem`) "Digit" "/Game/JamAssets/2DAssets/Numbers/0.0"))
      (:`Case_1`
        (`NiagaraFunctionLibrary.SetTextureObject` (`local.DigitSystem`) "Digit" "/Game/JamAssets/2DAssets/Numbers/1.1"))
      (:`Case_2`
        (`NiagaraFunctionLibrary.SetTextureObject` null "Digit" "/Game/JamAssets/2DAssets/Numbers/2.2"))
      (:`Case_3`
        (`NiagaraFunctionLibrary.SetTextureObject` null "Digit" "/Game/JamAssets/2DAssets/Numbers/3.3"))
      (:`Case_4`
        (`NiagaraFunctionLibrary.SetTextureObject` null "Digit" "/Game/JamAssets/2DAssets/Numbers/4.4"))
      (:`Case_5`
        (`NiagaraFunctionLibrary.SetTextureObject` null "Digit" "/Game/JamAssets/2DAssets/Numbers/5.5"))
      (:`Case_6`
        (`NiagaraFunctionLibrary.SetTextureObject` null "Digit" "/Game/JamAssets/2DAssets/Numbers/7.7"))
      (:`Case_7`
        (`NiagaraFunctionLibrary.SetTextureObject` null "Digit" "/Game/JamAssets/2DAssets/Numbers/8.8"))
      (:`Case_8`
        (`NiagaraFunctionLibrary.SetTextureObject` null "Digit" "/Game/JamAssets/2DAssets/Numbers/9.9"))
      (:`Case_9`
        (`NiagaraFunctionLibrary.SetTextureObject` null "Digit" "/Game/JamAssets/2DAssets/Numbers/9.9")))))

(fn `UserConstructionScript`)