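; BP_FloatHead is a floating-head enemy that turns toward the player and moves forward every tick without sweeping.
; Overlapping BP_Paint applies a fixed TickDamage, then spawns delayed floating text showing a random number from the player's damage range, unrelated to the damage applied, with a separately rolled color.
; AttackProjectile fires BP_EnemyProjectile along the player direction, but its only call in this graph is disconnected.
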(event `self.ReceiveBeginPlay`
  (bind _asbp_first_person_character (cast `/Game/JamAssets/Blueprints/BP_FirstPersonCharacter` (`GameplayStatics.GetPlayerPawn` 0)))
  (set `self.As BP First Person Character` _asbp_first_person_character))

(event `self.ReceiveTick`
  (params (DeltaSeconds :type "Float (single-precision)"))
  (bind _returnvalue (`self.K2_GetActorLocation`))
  (bind _returnvalue_2 (`self.K2_GetActorLocation` (`GameplayStatics.GetPlayerPawn` 0)))
  (`|ExecutionSequence`
    (:`then_0`
      (if (not (`self.IsTickeable`))
        (`KismetSystemLibrary.Delay` 0.8)
        (set `self.IsTickeable` true)))
    (:`then_1`
      (set `self.Player dir` (`KismetMathLibrary.GetDirectionUnitVector` _returnvalue _returnvalue_2))
      (`self.K2_SetActorRotation` (`KismetMathLibrary.RInterpTo` (`self.K2_GetActorRotation`) (`KismetMathLibrary.FindLookAtRotation` _returnvalue _returnvalue_2) (`GameplayStatics.GetWorldDeltaSeconds`)))
      (`SceneComponent.K2_AddWorldOffset` (`self.CapsuleComponent`) (* (`self.GetActorForwardVector`) (`self.MoveSpeed`)) false false))))

(event `AttackProjectile`
  (`|SpawnActorFromClass` "/Game/JamAssets/Blueprints/BP_EnemyProjectile.BP_EnemyProjectile_C" (`SceneComponent.K2_GetComponentToWorld` (`self.HeterogeneousVolume`)) "Undefined" "MultiplyWithRoot" null (`self.Player Dir`) (`self.Damage`) null))

(event `MakeDamage`
  (params (Location :type "Vector Structure") (Amount :type Integer) (Color :type "LinearColor Structure"))
  (`KismetSystemLibrary.Delay` 0.8)
  (`|SpawnActorFromClass` "/Game/JamAssets/Blueprints/HUDBP/BP_FloatingTextA.BP_FloatingTextA_C" (`self.GetTransform`) "Undefined" "MultiplyWithRoot" null Amount Color null))

(event `self.CapsuleComponent.OnComponentBeginOverlap`
  (params (OverlappedComponent :type "PrimitiveComponent Object Reference") (OtherActor :type "Actor Object Reference") (OtherComp :type "PrimitiveComponent Object Reference") (OtherBodyIndex :type Integer) (bFromSweep :type Boolean) (SweepResult :type "HitResult Structure (by ref)"))
  (bind _as_bp_first_person_character (`self.As BP First Person Character`))
  (bind _maxdamage (`JamCharacter.MaxDamage` _as_bp_first_person_character))
  (bind _returnvalue (`KismetMathLibrary.RandomIntegerInRange` (`JamCharacter.MinDamage` _as_bp_first_person_character) _maxdamage))
  (cast `/Game/JamAssets/Blueprints/BP_Paint` OtherActor)
  (`Tickeable.TickDamage` 35)
  (`/Engine/EditorBlueprintResources/StandardMacros.IsValid` self
    (:`Is Valid`
      (`self.MakeDamage` (0.0 0.0 0.0) _returnvalue (`KismetMathLibrary.LinearColorLerp` (struct :`R` 0.51255 :`G` 1.0 :`B` 0.47823 :`A` 1.0) (struct :`R` 1.0 :`A` 1.0) (`KismetMathLibrary.Conv_IntToDouble` (/ _returnvalue _maxdamage)))))))

(fn `UserConstructionScript`)