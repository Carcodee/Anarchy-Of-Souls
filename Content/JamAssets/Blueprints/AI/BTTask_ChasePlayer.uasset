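; Behavior Tree task that makes an AI pawn chase the first-person player character.
; While the player is falling, flying or in the IsCreating state, it uses a simple move to the player's XY at the pawn's own height.
; Otherwise it issues AIMoveTo on the player actor.
; Both branches finish successfully right after issuing the move, without waiting for arrival.
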(event `self.ReceiveExecuteAI`
  (params (OwnerController :type "AIController Object Reference") (ControlledPawn :type "Pawn Object Reference"))
  (bind (_returnvalue_x _returnvalue_y _returnvalue_z) (`KismetMathLibrary.BreakVector` (`Actor.K2_GetActorLocation` ControlledPawn)))
  (bind _returnvalue (`GameplayStatics.GetPlayerPawn` 0))
  (bind _as_bp_first_person_character (`self.As BP First Person Character`))
  (bind (_returnvalue_x_2 _returnvalue_y_2 _returnvalue_z_2) (`KismetMathLibrary.BreakVector` (`Actor.K2_GetActorLocation` _returnvalue)))
  (bind _charactermovement (`Character.CharacterMovement` _as_bp_first_person_character))
  (bind _iscreating (`/Game/JamAssets/Blueprints/BP_FirstPersonCharacter.IsCreating` _as_bp_first_person_character))
  (bind _asbp_first_person_character (cast `/Game/JamAssets/Blueprints/BP_FirstPersonCharacter` _returnvalue))
  (set `self.As BP First Person Character` _asbp_first_person_character)
  (set `self.Dest` (`KismetMathLibrary.MakeVector` _returnvalue_x_2 _returnvalue_y_2 _returnvalue_z))
  (if (or (`NavMovementComponent.IsFalling` _charactermovement) (`NavMovementComponent.IsFlying` _charactermovement) _iscreating (and _iscreating (!= (`KismetMathLibrary.FFloor` _returnvalue_z_2) (`KismetMathLibrary.FFloor` _returnvalue_z))))
    (`AIBlueprintHelperLibrary.SimpleMoveToLocation` OwnerController (`self.Dest`))
    (else
      (`|AIMoveTo` ControlledPawn (0.0 0.0 0.0) _returnvalue
        (:`then`
          _))))
  (`self.FinishExecute` true))